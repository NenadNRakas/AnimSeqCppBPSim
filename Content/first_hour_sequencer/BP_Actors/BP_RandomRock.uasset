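; BP_RandomRock is a short-lived physics rock actor that takes a random shape.
; Its construction script picks a random mesh from the Meshes array and enables physics simulation on it.
; On BeginPlay, a timer with a random delay of a few seconds calls die, which destroys the actor.
; The small and large rock scale variables are unused.
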(event Custom|die
  (Actor|DestroyActor))

(event EventBeginPlay
  (Utilities|Time|SetTimerbyFunctionName 0 "die" (Math|Random|RandomFloatinRange 3.0 8.0)))

(fn ConstructionScript
  (bind _meshes (Variables|Default|GetMeshes))
  (Components|StaticMesh|SetStaticMesh (Variables|Default|GetStaticMesh) (Utilities|Array|Get(acopy) _meshes (Math|Random|RandomInteger (Utilities|Array|Length _meshes))))
  (Physics|SetSimulatePhysics (Variables|Default|GetStaticMesh) true))